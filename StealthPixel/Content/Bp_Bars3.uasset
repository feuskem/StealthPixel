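; Bp_Bars3 is a Paper2D barred-gate actor that opens once for a player character holding a key.
; Overlapping the Kapi component casts the actor to BP_2DCharacter and checks its KEY flag.
; It then plays the flipbook, which is stopped at BeginPlay, for a short fixed delay, freezes it and disables the Box collision.
; NewVar latches afterwards, so later overlaps do nothing.
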(event OnComponentBeginOverlap(Kapi)
  (params (OverlappedComponent :type Primitive%20Component%20Object%20Reference) (OtherActor :type Actor%20Object%20Reference) (OtherComp :type Primitive%20Component%20Object%20Reference) (OtherBodyIndex :type Integer) (bFromSweep :type Boolean) (SweepResult :type Hit%20Result%20Structure%20%28by%20ref%29))
  (bind _paperflipbook (Variables|Default|GetPaperFlipbook))
  (bind _asbp_2dcharacter (Utilities|Casting|CastToBP_2DCharacter OtherActor))
  (if (not (Variables|Default|GetNewVar))
    (if (Variables|/Game/Character/BP_2DCharacter.BP_2DCharacter_C|GetKEY _asbp_2dcharacter)
      (Audio|Components|Audio|Play _paperflipbook)
      (Utilities|FlowControl|Delay 0.4)
      (Audio|Components|Audio|Stop _paperflipbook)
      (Collision|SetCollisionEnabled (Variables|Default|GetBox) "NoCollision")
      (Variables|Default|SetNewVar true))))

(event EventBeginPlay
  (Audio|Components|Audio|Stop (Variables|Default|GetPaperFlipbook)))

(event Collision|EventActorBeginOverlap
  (params (OtherActor :type Actor%20Object%20Reference)))

(event EventTick
  (params (DeltaSeconds :type Float%20%28single-precision%29)))

(fn ConstructionScript)