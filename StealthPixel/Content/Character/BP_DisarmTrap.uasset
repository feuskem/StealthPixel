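; BP_DisarmTrap is a trap actor that temporarily disarms any BP_2DEnemyBase overlapping its static mesh.
; On overlap it sets the enemy's IsDisarmed blackboard key, hides its Paper2D visuals and briefly plays a trigger flipbook.
; After fixed delays it clears the key and destroys itself, leaving the DisarmingDuration variable unused.
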(event OnComponentBeginOverlap(StaticMesh)
  (params (OverlappedComponent :type Primitive%20Component%20Object%20Reference) (OtherActor :type Actor%20Object%20Reference) (OtherComp :type Primitive%20Component%20Object%20Reference) (OtherBodyIndex :type Integer) (bFromSweep :type Boolean) (SweepResult :type Hit%20Result%20Structure%20%28by%20ref%29))
  (bind _returnvalue (Utilities|Name|MakeLiteralName "IsDisarmed"))
  (bind _paperflipbook (Variables|Default|GetPaperFlipbook))
  (bind _asbp_2denemy_base (Utilities|Casting|CastToBP_2DEnemyBase OtherActor))
  (AI|Components|Blackboard|SetValueasBool (AI|GetBlackboard (AI|GetAIController _asbp_2denemy_base)) _returnvalue true)
  (Development|SetHiddeninGame (Variables|Default|GetPaperFlipbook) true false)
  (Development|SetHiddeninGame (Variables|Default|GetPaperFlipbook) false false)
  (Components|Timeline|PlayfromStart _paperflipbook)
  (Utilities|FlowControl|Delay 0.7)
  (Audio|Components|Audio|Stop (Variables|Default|GetPaperFlipbook))
  (Development|SetHiddeninGame _paperflipbook true false)
  (Utilities|FlowControl|Delay 4.0)
  (AI|Components|Blackboard|SetValueasBool (AI|GetBlackboard (AI|GetAIController _asbp_2denemy_base)) _returnvalue false)
  (Actor|DestroyActor))

(event EventBeginPlay
  (Rendering|Material|SetMaterial (Variables|Default|GetStaticMesh) 0 "/DatasmithContent/Materials/AliasReference.AliasReference"))

(event Collision|EventActorBeginOverlap
  (params (OtherActor :type Actor%20Object%20Reference)))

(event EventTick
  (params (DeltaSeconds :type Float%20%28single-precision%29)))

(fn ConstructionScript)