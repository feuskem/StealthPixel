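; BP_Noise is a one-shot sprite noisemaker that emits an AI-audible noise when the 2D character or an arrow touches it.
; The sprite's overlap event casts to BP_2DCharacter or BP_CommonArrow, then after a brief delay calls MakeNoise, plays a wood landing sound and destroys the actor.
; Arrow hits credit the noise to the player character cached on BeginPlay, so either trigger names the character as instigator.
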(event OnComponentBeginOverlap(PaperSprite)
  (params (OverlappedComponent :type Primitive%20Component%20Object%20Reference) (OtherActor :type Actor%20Object%20Reference) (OtherComp :type Primitive%20Component%20Object%20Reference) (OtherBodyIndex :type Integer) (bFromSweep :type Boolean) (SweepResult :type Hit%20Result%20Structure%20%28by%20ref%29))
  (bind _returnvalue (Transformation|GetActorLocation))
  (bind _returnvalue_2 (Transformation|GetActorLocation))
  (Utilities|FlowControl|Sequence
    (:then_0
      (bind _asbp_2dcharacter (Utilities|Casting|CastToBP_2DCharacter OtherActor))
      (Utilities|FlowControl|Delay 0.2)
      (Class|Actor|MakeNoise 1.0 _asbp_2dcharacter _returnvalue_2 0.0 "None")
      (Audio|PlaySoundatLocation "/Game/Character/422869__ipaddeh__jump_landing_wood_02.422869__ipaddeh__jump_landing_wood_02" _returnvalue_2 "0, 0, 0" 1.0 1.0 0.0 0 0 0 0)
      (Actor|DestroyActor))
    (:then_1
      (Utilities|Casting|CastToBP_CommonArrow OtherActor)
      (Utilities|FlowControl|Delay 0.01)
      (Class|Actor|MakeNoise 1.0 (Variables|Default|GetNewVar) _returnvalue 0.0 "None")
      (Audio|PlaySoundatLocation "/Game/Character/422869__ipaddeh__jump_landing_wood_02.422869__ipaddeh__jump_landing_wood_02" _returnvalue "0, 0, 0" 1.0 1.0 0.0 0 0 0 0)
      (Actor|DestroyActor))))

(event EventBeginPlay
  (bind _returnvalue (Actor|GetActorOfClass "/Game/Character/BP_2DCharacter.BP_2DCharacter_C"))
  (Variables|Default|SetNewVar _returnvalue))

(event Collision|EventActorBeginOverlap
  (params (OtherActor :type Actor%20Object%20Reference)))

(event EventTick
  (params (DeltaSeconds :type Float%20%28single-precision%29)))

(fn ConstructionScript)