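; Player character for a 2D sprite game, with Enhanced Input movement and roll, inventory, item interaction, trap placement and health.
; Number keys toggle dagger or crossbow; the crossbow aims by mouse, loads over time and makes noise on firing, while the dagger destroys an overlapping enemy.
; Timelines shift the camera with movement.
; Looping timers regenerate stamina and sphere-trace from camera to sprite, swapping its material when blocked.
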(event OnComponentBeginOverlap(Capsule)
  (params (OverlappedComponent :type Primitive%20Component%20Object%20Reference) (OtherActor :type Actor%20Object%20Reference) (OtherComp :type Primitive%20Component%20Object%20Reference) (OtherBodyIndex :type Integer) (bFromSweep :type Boolean) (SweepResult :type Hit%20Result%20Structure%20%28by%20ref%29))
  (bind _asbp_2denemy_base (Utilities|Casting|CastToBP_2DEnemyBase OtherActor))
  (Variables|Default|SetAs%20BP%202DEnemy%20Base _asbp_2denemy_base)
  (Variables|Default|SetIsThereEnemyInRange true))

(event OnComponentEndOverlap(Capsule)
  (params (OverlappedComponent :type Primitive%20Component%20Object%20Reference) (OtherActor :type Actor%20Object%20Reference) (OtherComp :type Primitive%20Component%20Object%20Reference) (OtherBodyIndex :type Integer))
  (Utilities|Casting|CastToBP_2DEnemyBase OtherActor)
  (Variables|Default|SetIsThereEnemyInRange false))

(event Custom|Refresh
  (if (not (Variables|Default|GetInv%20Close))
    (Widget|RemovefromParent (stale _returnvalue))
    (bind _use_menu (Variables|/Game/Inventory/InventorySystem.InventorySystem_C|GetUse%20Menu (Variables|Default|GetInventorySystem))
      (:then
        (Widget|RemovefromParent _use_menu))
      (:else
        _))
    (bind _returnvalue (UserInterface|CreateWidget "/Game/Inventory/Inventory_Widget.Inventory_Widget_C"))
    (UserInterface|Viewport|AddtoViewport _returnvalue 0)
    (Variables|Default|SetInv%20Close false)))

(event Custom|CursorChange
  (if true
    (Utilities|FlowControl|Delay 0.1)))

(event Custom|CheckWalls
  (bind _wall (Variables|Default|GetWall))
  (Utilities|Time|SetTimerbyEvent (delegate Custom|CheckWalls) 0.1 true)
  (bind _outhit (Collision|SphereTraceByChannel (Transformation|GetWorldLocation (Variables|Default|GetCamera)) (Transformation|GetWorldLocation (Variables|Default|GetSprite)) 3e+01 "TraceTypeQuery4" false 0 "None" false))
  (if (== (Variables|Default|GetCapsuleComponent) (.HitComponent (Collision|BreakHitResult _outhit)))
    (for _array_element _wall
      (Rendering|Material|SetMaterial (Variables|Default|GetSprite) 0 "/Paper2D/MaskedUnlitSpriteMaterial.MaskedUnlitSpriteMaterial")
      (Utilities|Array|Clear _wall))
    (else
      (Utilities|Array|Add (Variables|Default|GetWall) (.HitComponent (Collision|BreakHitResult _outhit)))
      (for _array_element_2 (Variables|Default|GetWall)
        (if (== _array_element_2 (.HitComponent (Collision|BreakHitResult _outhit)))
          (Rendering|Material|SetMaterial (Variables|Default|GetSprite) 0 "/Game/AA.AA")
          (else
            (Rendering|Material|SetMaterial (Variables|Default|GetSprite) 0 "/Paper2D/MaskedUnlitSpriteMaterial.MaskedUnlitSpriteMaterial")
            (Utilities|Array|RemoveItem (Variables|Default|GetWall) _array_element_2)))))))

(event Custom|Stamina
  (Utilities|Time|SetTimerbyEvent (delegate Custom|Stamina) 0.1 true)
  (if (<= (Variables|Default|GetCurrentStamina) 0.0)
    (Utilities|FlowControl|Delay 0.5))
  (if (not (== (Variables|Default|GetMaxStamina) (Variables|Default|GetCurrentStamina)))
    (Variables|Default|SetCurrentStamina (+ (Variables|Default|GetCurrentStamina) 1.0))))

(event Input|EnhancedActionEvents|EnhancedInputActionIA_Move
  (params (ActionValue :type Vector%202D%20Structure) (ElapsedSeconds :type Float%20%28double-precision%29) (TriggeredSeconds :type Float%20%28double-precision%29) (InputAction :type Input%20Action%20Object%20Reference :default "/Game/Input/IA_Move.IA_Move"))
  (:Triggered
    (Pawn|Input|AddMovementInput "1.000000,0.000000,0.000000" (.x ActionValue) false)
    (Pawn|Input|AddMovementInput "0.000000,-1.000000,0.000000" (.y ActionValue) false)
    (Variables|Default|SetDirectioanlity (Math|Vector2D|MakeVector2D (.x ActionValue) (.y ActionValue))))
  (:Started
    (Utilities|FlowControl|Sequence
      (:then_0
        (if (== (.y ActionValue) 1.0) :!label _label
          (bind _newtrack_0 (Timeline|CameraMovementUp Play)
            (:Update
              (Components|MoveComponentTo (Variables|Default|GetCamera) (Math|Vector|MakeVector 0.0 0.0 _newtrack_0) "0, 0, 0" false false 0.2 true)))))
      (:then_1
        (if (== (.y ActionValue) -1.0) :!label _label_2
          (bind _newtrack_0_2 (Timeline|Timeline Play)
            (:Update
              (Components|MoveComponentTo (Variables|Default|GetCamera) (Math|Vector|MakeVector 0.0 0.0 _newtrack_0_2) "0, 0, 0" false false 0.2 true)))))
      (:then_2
        (if (== (.x ActionValue) -1.0) :!label _label_3
          (bind _newtrack_0_3 (Timeline|Timeline_0 Play)
            (:Update
              (Components|MoveComponentTo (Variables|Default|GetCamera) (Math|Vector|MakeVector 0.0 _newtrack_0_3 0.0) "0, 0, 0" false false 0.2 true)))))
      (:then_3
        (if (== (.x ActionValue) 1.0) :!label _label_4
          (bind _newtrack_0_4 (Timeline|Timeline_1 Play)
            (:Update
              (Components|MoveComponentTo (Variables|Default|GetCamera) (Math|Vector|MakeVector 0.0 _newtrack_0_4 0.0) "0, 0, 0" false true 0.2 true)))))
      (:then_4
        (Variables|Default|SetIsHoldingMove true))))
  (:Ongoing
    (Utilities|FlowControl|Sequence
      (:then_0
        (goto _label))
      (:then_1
        (goto _label_2))
      (:then_2
        (goto _label_3))
      (:then_3
        (goto _label_4))))
  (:Completed
    (Utilities|FlowControl|Sequence
      (:then_0
        (Variables|Default|SetIsHoldingMove false)))))

(event Input|EnhancedActionEvents|EnhancedInputActionIA_Shoot
  (params (ActionValue :type Boolean) (ElapsedSeconds :type Float%20%28double-precision%29) (TriggeredSeconds :type Float%20%28double-precision%29) (InputAction :type Input%20Action%20Object%20Reference :default "/Game/Input/IA_Shoot.IA_Shoot"))
  (:Triggered
    (Variables|Default|SetHasRangedWeapon true)
    (Variables|Default|SetCbAim true))
  (:Completed
    (Variables|Default|SetHasRangedWeapon false)
    (Variables|Default|SetCbAim false)))

(event Input|EnhancedActionEvents|EnhancedInputActionIA_Roll
  (params (ActionValue :type Boolean) (ElapsedSeconds :type Float%20%28double-precision%29) (TriggeredSeconds :type Float%20%28double-precision%29) (InputAction :type Input%20Action%20Object%20Reference :default "/Game/Input/IA_Roll.IA_Roll"))
  (bind _directioanlity (Variables|Default|GetDirectioanlity))
  (:Triggered
    (if true
      (bind _distancemultiplier (Timeline|RollMovement PlayFromStart)
        (:Update
          _)
        (:Finished
          _))
      (Variables|/Script/Engine.MovementComponent|SetVelocity (Variables|Character|GetCharacterMovement) (Math|Vector|MakeVector (* (* (.x _directioanlity) 1e+03) _distancemultiplier) (* (* (.y _directioanlity) -1e+03) _distancemultiplier) 0.0))))
  (:Started
    (if true
      (Class|PaperZDAnimInstance|JumptoNode (Variables|/Script/PaperZD.PaperZDAnimationComponent|GetAnimInstance (Variables|Default|GetAnimationComponent)) "Roll" ""))))

(event EventBeginPlay
  (bind _asplayer_controller (Utilities|Casting|CastToPlayerController (Pawn|GetController)))
  (Input|AddMappingContext (PlayerController|LocalPlayerSubsystems|GetEnhancedInputLocalPlayerSubsystem _asplayer_controller) "/Game/Input/IMC_2D.IMC_2D" 0 "(bIgnoreAllPressedKeysUntilRelease=True,bForceImmediately=False,bNotifyUserSettings=False)")
  (bind _returnvalue (UserInterface|CreateWidget "/Game/Widgets/W_HUD.W_HUD_C"))
  (UserInterface|Viewport|AddtoViewport _returnvalue 0)
  (bind _returnvalue_2 (Actor|GetActorOfClass "/Game/OBSTACEL.OBSTACEL_C"))
  (Variables|Default|SetNewVar _returnvalue_2)
  (CallFunction|CheckWalls)
  (bind _returnvalue_3 (Actor|GetActorOfClass "/Game/Character/BP_Mahlukat.BP_Mahlukat_C"))
  (Variables|Default|SetMahllukat _returnvalue_3)
  (CallFunction|Stamina)
  (Actor|GetActorOfClass "/Game/Enemies/BP_2DEnemy_Melee.BP_2DEnemy_Melee_C"))

(event Collision|EventActorBeginOverlap
  (params (OtherActor :type Actor%20Object%20Reference)))

(event EventTick
  (params (DeltaSeconds :type Float%20%28single-precision%29))
  (bind _returnvalue (Game|GetPlayerController 0))
  (bind (_worldlocation _worlddirection) (Game|Player|ConvertMouseLocationToWorldSpace _returnvalue))
  (Utilities|FlowControl|Sequence
    (:then_0
      (if (not (Variables|Default|GetDead))
        (if (<= (Variables|Default|GetHealth) 0.0)
          (Variables|Default|SetDead true)
          (Actor|DestroyActor self))))
    (:then_1
      (if (or false (Variables|Default|GetHasRangedWeapon))
        ;[1 1 1] Ranged Weapon
        (Transformation|SetRelativeRotation (Variables|Default|GetRotationPoint) (Math|Rotator|MakeRotator 0.0 (* (.yaw (Math|Rotator|FindLookatRotation _worldlocation (+ _worldlocation (* _worlddirection 1e+03)))) -1.0) 0.0) false false)
        (CallFunction|RotateCharacter)))))

(event Game|Damage|EventAnyDamage
  (params (Damage :type Float%20%28single-precision%29) (DamageType :type Damage%20Type%20Object%20Reference) (InstigatedBy :type Controller%20Object%20Reference) (DamageCauser :type Actor%20Object%20Reference))
  (Variables|Default|SetHealth (- (Variables|Default|GetHealth) Damage))
  (Development|PrintString (Utilities|String|ToString(Float) (Variables|Default|GetHealth))))

(event Input|MouseEvents|LeftMouseButton
  (params (Key :type Key%20Structure :default "None"))
  (bind _rotationpoint (Variables|Default|GetRotationPoint))
  (bind _returnvalue (Transformation|GetWorldTransform _rotationpoint))
  (:Pressed
    (if (Variables|Default|GetIsHoldingCrossbow)
      (if (Variables|Default|GetHasRangedWeapon)
        (if (Variables|Default|GetLoaded)
          (Game|SpawnActorfromClass (Variables|Default|GetProjectileClass) (Math|Transform|MakeTransform (Math|Vector|MakeVector (.x (.location _returnvalue)) (.y (.location _returnvalue)) 77.55) (Math|Rotator|MakeRotator (.roll (.rotation _returnvalue)) 0.0 (.yaw (.rotation _returnvalue))) (.scale _returnvalue)) "AdjustIfPossibleButDontSpawnIfColliding" "MultiplyWithRoot" 0 0)
          (Variables|Default|SetLoaded false)
          (Variables|Default|SetLoadTime 0.0)
          (Class|Actor|MakeNoise 1.0 self (Transformation|GetActorLocation) 0.0 "None")
          (else
            (Variables|Default|SetLoadTime (+ (Variables|Default|GetLoadTime) 0.1) :!label _label)
            (Development|PrintString (Utilities|String|ToString(Float) (Variables|Default|GetLoadTime)))
            (if (and (== (Variables|Default|GetLoadTime) 0.5) (== (Variables|Default|GetProjectileClass) "/Game/Weapons/BP_CommonArrow.BP_CommonArrow_C"))
              (Variables|Default|SetLoaded true)
              (elif (and (>= (Variables|Default|GetLoadTime) 0.2) (== (Variables|Default|GetProjectileClass) "/Game/Weapons/BP_QuickArrow.BP_QuickArrow_C"))
                (Variables|Default|SetLoaded true)
                (else
                  (Utilities|FlowControl|Delay 0.1)
                  (goto _label))))))
        (else
          (if (Variables|Default|GetIsHoldingDagger) :!label _label_2
            (if (Variables|Default|GetMeleeMode)
              (Variables|Default|SetMeleeMode false)
              (Class|PaperZDAnimInstance|JumptoNode (Variables|/Script/PaperZD.PaperZDAnimationComponent|GetAnimInstance (Variables|Default|GetAnimationComponent)) "Attack" "")
              (Utilities|FlowControl|Sequence
                (:then_0
                  (if (Variables|Default|GetIsThereEnemyInRange)
                    (Actor|DestroyActor (Variables|Default|GetAs%20BP%202DEnemy%20Base))
                    (Audio|PlaySound2D "/Game/Character/518883__beezlefm__simple-slash-attack-sound.518883__beezlefm__simple-slash-attack-sound" 1.0 1.0 0.0 0 0)))
                (:then_1
                  (Utilities|FlowControl|Delay 0.5)
                  (Variables|Default|SetMeleeMode true))
                (:then_2
                  (bind _newtrack_0 (Timeline|Timeline_3 PlayFromStart)
                    (:Update
                      _)
                    (:Finished
                      _))
                  (Variables|/Script/Engine.MovementComponent|SetVelocity (Variables|Character|GetCharacterMovement) (Math|Conversions|ToVector(Float) _newtrack_0))))))))
      (else
        (goto _label_2)))))

(event Input|KeyboardEvents|Tab
  (params (Key :type Key%20Structure :default "None"))
  (:Pressed
    (if (Variables|Default|GetInv%20Close)
      (bind _returnvalue (UserInterface|CreateWidget "/Game/Inventory/Inventory_Widget.Inventory_Widget_C"))
      (UserInterface|Viewport|AddtoViewport _returnvalue 0)
      (Variables|Default|SetInv%20Close false)
      (else
        (Widget|RemovefromParent _returnvalue)
        (bind _use_menu (Variables|/Game/Inventory/InventorySystem.InventorySystem_C|GetUse%20Menu (Variables|Default|GetInventorySystem))
          (:then
            (Widget|RemovefromParent _use_menu))
          (:else
            _))
        (Variables|Default|SetInv%20Close true)))))

(event Input|KeyboardEvents|9
  (params (Key :type Key%20Structure :default "None"))
  (:Pressed
    (bind _returnvalue (Actor|GetActorOfClass "/Game/Enemies/BP_2DEnemyBase.BP_2DEnemyBase_C"))
    (bind _asaic_enemy_base (Utilities|Casting|CastToAIC_Enemy_Base (AI|GetAIController _returnvalue)))
    (Utilities|FlowControl|FlipFlop
      (:A
        (Default|SetStateasAttacking _asaic_enemy_base self))
      (:B
        (Default|SetStateasPassive _asaic_enemy_base)))))

(event Input|KeyboardEvents|2
  (params (Key :type Key%20Structure :default "None"))
  (:Pressed
    (Utilities|FlowControl|FlipFlop
      (:A
        (Variables|Default|SetIsHoldingCrossbow true)
        (Variables|Default|SetIsHoldingDagger false)
        (Class|PaperZDAnimInstance|JumptoNode (Variables|/Script/PaperZD.PaperZDAnimationComponent|GetAnimInstance (Variables|Default|GetAnimationComponent)) "Crossbow" ""))
      (:B
        (Variables|Default|SetIsHoldingCrossbow false)
        (Variables|Default|SetIsHoldingDagger false)
        (Class|PaperZDAnimInstance|JumptoNode (Variables|/Script/PaperZD.PaperZDAnimationComponent|GetAnimInstance (Variables|Default|GetAnimationComponent)) "Holster" "")))))

(event Input|KeyboardEvents|L
  (params (Key :type Key%20Structure :default "None"))
  (bind _returnvalue (Transformation|GetActorLocation))
  (:Pressed
    (Class|Actor|MakeNoise 1.0 self _returnvalue 0.0 "None")
    (Audio|PlaySoundatLocation "/Engine/EngineSounds/1kSineTonePing.1kSineTonePing" _returnvalue "0, 0, 0" 1.0 1.0 0.0 0 0 0 0)))

(event Input|KeyboardEvents|1
  (params (Key :type Key%20Structure :default "None"))
  (bind _animationcomponent (Variables|Default|GetAnimationComponent))
  (bind _animinstance (Variables|/Script/PaperZD.PaperZDAnimationComponent|GetAnimInstance _animationcomponent))
  (:Pressed
    (Utilities|FlowControl|FlipFlop
      (:A
        (Variables|Default|SetIsHoldingDagger true)
        (Variables|Default|SetIsHoldingCrossbow false)
        (Class|PaperZDAnimInstance|JumptoNode _animinstance "DaggerIdle" ""))
      (:B
        (Variables|Default|SetIsHoldingDagger false)
        (Variables|Default|SetIsHoldingCrossbow false)
        (Class|PaperZDAnimInstance|JumptoNode _animinstance "Holster" "")))))

(event Input|KeyboardEvents|E
  (params (Key :type Key%20Structure :default "None"))
  (bind _returnvalue (Transformation|GetActorLocation))
  (:Pressed
    (bind (_outhit _returnvalue_2) (Collision|SphereTraceByChannel _returnvalue _returnvalue 1.2e+02 "TraceTypeQuery6" false 0 "ForDuration"))
    (if _returnvalue_2
      (bind _asitem (Utilities|Casting|CastToItem (.HitActor (Collision|BreakHitResult _outhit))))
      (Default|Interact _asitem))))

(event Input|KeyboardEvents|P
  (params (Key :type Key%20Structure :default "None"))
  (bind _returnvalue (Game|GetPlayerCharacter 0))
  (bind _returnvalue_2 (Transformation|GetActorLocation _returnvalue))
  (bind _returnvalue_3 (Transformation|GetActorForwardVector _returnvalue))
  (bind _returnvalue_4 (Transformation|GetActorUpVector _returnvalue))
  (bind _returnvalue_5 (Transformation|GetActorRightVector _returnvalue))
  (bind _returnvalue_6 (* _returnvalue_3 85.0))
  (bind _returnvalue_7 (* _returnvalue_5 1e+02))
  (bind _returnvalue_8 (* _returnvalue_4 75.0))
  (bind _returnvalue_9 (+ _returnvalue_2 _returnvalue_6 _returnvalue_8 _returnvalue_7))
  (:Pressed
    (Game|SpawnActorfromClass "/Game/Character/BP_ParalysisTrap.BP_ParalysisTrap_C" (Math|Transform|MakeTransform (Math|Vector|MakeVector (.x _returnvalue_9) (.y _returnvalue_9) 0.5) "0, 0, 0" "1.000000,1.000000,1.000000") "AdjustIfPossibleButAlwaysSpawn" "MultiplyWithRoot" 0 0)))

(event Input|KeyboardEvents|LeftShift
  (params (Key :type Key%20Structure :default "None"))
  (:Released
    (Variables|Default|SetMeleeMode false)
    (Variables|Default|SetCursorMode 0)))

(event Input|KeyboardEvents|SpaceBar
  (params (Key :type Key%20Structure :default "None")))

(event Input|KeyboardEvents|3
  (params (Key :type Key%20Structure :default "None"))
  (:Pressed
    (Variables|Default|SetProjectileClass "/Game/Weapons/BP_QuickArrow.BP_QuickArrow_C")))

(event Input|KeyboardEvents|W
  (params (Key :type Key%20Structure :default "None"))
  (:Pressed
    (Transformation|SetRelativeRotation (Variables|Default|GetRotationPoint) "90.000000,0.000000,0.000000" false false)
    (Development|PrintString "Hello")))

(event Input|KeyboardEvents|S
  (params (Key :type Key%20Structure :default "None"))
  (:Pressed
    (Transformation|SetRelativeRotation (Variables|Default|GetRotationPoint) "270.000000,0.000000,0.000000" false false)))

(event Input|KeyboardEvents|A
  (params (Key :type Key%20Structure :default "None"))
  (:Pressed
    (Transformation|SetRelativeRotation (Variables|Default|GetRotationPoint) "180.000000,0.000000,0.000000" false false)))

(event Input|KeyboardEvents|D
  (params (Key :type Key%20Structure :default "None"))
  (:Pressed
    (Transformation|SetRelativeRotation (Variables|Default|GetRotationPoint) "0, 0, 0" false false)))

(event Input|KeyboardEvents|LeftCtrl
  (params (Key :type Key%20Structure :default "None"))
  (:Pressed
    (Utilities|FlowControl|FlipFlop
      (:A
        (Character|Crouch))
      (:B
        (Character|UnCrouch)))))

(fn ConstructionScript)

(fn IsStuck
  (return (and (Variables|Default|GetIsHoldingMove) (< (Math|Vector|VectorLength (Transformation|GetVelocity)) (Variables|Default|GetStuckTrehshlod)))))

(fn RotateCharacter
  (bind _rotationpoint (Variables|Default|GetRotationPoint))
  (bind _relativerotation (Variables|/Script/Engine.SceneComponent|GetRelativeRotation _rotationpoint))
  (if (and (< (.pitch _relativerotation) -45.0) (> (.pitch _relativerotation) -135.0))
    (Variables|Default|SetDirectioanlity "(X=0.000000,Y=-1.000000)")
    (elif (and (> (.pitch _relativerotation) 45.0) (< (.pitch _relativerotation) 135.0))
      (Variables|Default|SetDirectioanlity "(X=0.000000,Y=1.000000)")
      (elif (or (Math|Float|InRange(Float) (.roll _relativerotation) 1.6e+02 2e+02) (Math|Float|InRange(Float) (.roll _relativerotation) -2e+02 -1.6e+02))
        (Variables|Default|SetDirectioanlity "(X=-1.000000,Y=0.000000)")
        (elif (and (> (.pitch _relativerotation) -45.0) (< (.pitch _relativerotation) 45.0))
          (Variables|Default|SetDirectioanlity "(X=1.000000,Y=0.000000)"))))))