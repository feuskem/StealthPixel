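; BP_ParalysisTrap is a 2D trap that briefly freezes an enemy that walks into it, then destroys itself.
; When a BP_2DEnemyBase overlaps its Sphere, it sets the IsFreezed key on that enemy's AI blackboard and clears it a fraction of a second later.
; It then swaps its Paper sprite to the closed-trap image and destroys the actor after a short delay.
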(event OnComponentBeginOverlap(Sphere)
  (params (OverlappedComponent :type Primitive%20Component%20Object%20Reference) (OtherActor :type Actor%20Object%20Reference) (OtherComp :type Primitive%20Component%20Object%20Reference) (OtherBodyIndex :type Integer) (bFromSweep :type Boolean) (SweepResult :type Hit%20Result%20Structure%20%28by%20ref%29))
  (bind _asbp_2denemy_base (Utilities|Casting|CastToBP_2DEnemyBase OtherActor))
  (AI|Components|Blackboard|SetValueasBool (AI|GetBlackboard (AI|GetAIController _asbp_2denemy_base)) (Utilities|Name|MakeLiteralName "IsFreezed") true)
  (Utilities|FlowControl|Delay 0.1)
  (AI|Components|Blackboard|SetValueasBool (AI|GetBlackboard (AI|GetAIController _asbp_2denemy_base)) (Utilities|Name|MakeLiteralName "IsFreezed") false)
  (Rendering|Components|Sprite|SetSprite (Variables|Default|GetPaperSprite) "/Game/Sprites/Traps/Paralysis/trapclosed_Sprite.trapclosed_Sprite")
  (Utilities|FlowControl|Delay 2.0)
  (Actor|DestroyActor))

(event EventBeginPlay)

(event Collision|EventActorBeginOverlap
  (params (OtherActor :type Actor%20Object%20Reference)))

(event EventTick
  (params (DeltaSeconds :type Float%20%28single-precision%29)))

(fn ConstructionScript)