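; Barrier actor that opens once the player completes the ranged tutorial.
; BeginPlay stops the flipbook, caches the BP_2DCharacter pawn and starts a looping timer on the Close event to poll its HasCompletedRangedTut flag.
; When the flag is set, the flipbook plays briefly and stops, then the Box collision is disabled and the timer is paused.
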(event Custom|Close
  (bind _paperflipbook (Variables|Default|GetPaperFlipbook))
  (bind _returnvalue (Utilities|Time|SetTimerbyEvent (delegate Custom|Close) 0.1 true))
  (if (Variables|/Game/Character/BP_2DCharacter.BP_2DCharacter_C|GetHasCompletedRangedTut (stale EventBeginPlay _asbp_2dcharacter))
    (Audio|Components|Audio|Play _paperflipbook)
    (Utilities|FlowControl|Delay 0.4)
    (Audio|Components|Audio|Stop _paperflipbook)
    (Collision|SetCollisionEnabled (Variables|Default|GetBox) "NoCollision")
    (Utilities|Time|PauseTimerbyHandle _returnvalue)))

(event EventBeginPlay
  (bind _paperflipbook (Variables|Default|GetPaperFlipbook))
  (Audio|Components|Audio|Stop (Variables|Default|GetPaperFlipbook))
  (bind _asbp_2dcharacter (Utilities|Casting|CastToBP_2DCharacter (Game|Player|GetPlayerPawn 0)))
  (bind _returnvalue (Utilities|Time|SetTimerbyEvent (delegate Custom|Close) 0.1 true))
  (if (Variables|/Game/Character/BP_2DCharacter.BP_2DCharacter_C|GetHasCompletedRangedTut _asbp_2dcharacter)
    (Audio|Components|Audio|Play _paperflipbook)
    (Utilities|FlowControl|Delay 0.4)
    (Audio|Components|Audio|Stop _paperflipbook)
    (Collision|SetCollisionEnabled (Variables|Default|GetBox) "NoCollision")
    (Utilities|Time|PauseTimerbyHandle _returnvalue)))

(event Collision|EventActorBeginOverlap
  (params (OtherActor :type Actor%20Object%20Reference)))

(event EventTick
  (params (DeltaSeconds :type Float%20%28single-precision%29)))

(fn ConstructionScript)