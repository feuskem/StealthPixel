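; Ranged 2D enemy that attacks by summoning melee minions and destroys itself when health reaches zero.
; Attack waits briefly, picks random reachable navmesh coordinates nearby at a fixed height, spawns two BP_2DEnemy_Melee actors, then signals attack end.
; It also supplies movement speeds per state and ideal attack and defend ranges.
; Two further spawns and manual controller possession are left unwired.
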(event EventBeginPlay
  (|CallParentFunction)
  (bind _returnvalue (Actor|GetActorOfClass "/Script/NavigationSystem.NavigationData"))
  (Variables|Default|SetNavData _returnvalue)
  (bind _returnvalue_2 (Actor|GetActorOfClass "/Game/Enemies/AI/AIC_Enemy_Base.AIC_Enemy_Base_C"))
  (Variables|Default|SetNewVar_0_0 _returnvalue_2))

(event Collision|EventActorBeginOverlap
  (params (OtherActor :type Actor%20Object%20Reference)))

(event EventTick
  (params (DeltaSeconds :type Float%20%28single-precision%29))
  (|CallParentFunction 0.0))

(event EventAttack
  (bind _returnvalue (Transformation|GetActorLocation))
  (bind _randomlocation (AI|Navigation|GetRandomReachablePointinRadius (Math|Vector|MakeVector (.x _returnvalue) (.y _returnvalue) 5e+01) 5e+02 0 0))
  (bind _randomlocation_2 (AI|Navigation|GetRandomReachablePointinRadius (Math|Vector|MakeVector (.x _returnvalue) (.y _returnvalue) 5e+01) 5e+02 0 0))
  (bind _randomlocation_3 (AI|Navigation|GetRandomReachablePointinRadius (Math|Vector|MakeVector (.x _returnvalue) (.y _returnvalue) 5e+01) 5e+02 0 0))
  (bind _randomlocation_4 (AI|Navigation|GetRandomReachablePointinRadius (Math|Vector|MakeVector (.x _returnvalue) (.y _returnvalue) 5e+01) 5e+02 0 0))
  (Utilities|FlowControl|Delay 0.2)
  (bind _output_get (Variables|Default|SetSpawnLocation1 (Math|Vector|MakeVector (.x _randomlocation_2) (.y _randomlocation_2) 5e+01)))
  (bind _output_get_2 (Variables|Default|SetSpawnLocation2 (Math|Vector|MakeVector (.x _randomlocation_3) (.y _randomlocation_3) 5e+01)))
  (bind _output_get_3 (Variables|Default|SetSpawnLocation3 (Math|Vector|MakeVector (.x _randomlocation_4) (.y _randomlocation_4) 5e+01)))
  (bind _output_get_4 (Variables|Default|SetSpawnLocation4 (Math|Vector|MakeVector (.x _randomlocation) (.y _randomlocation) 5e+01)))
  (Utilities|FlowControl|Sequence
    (:then_0
      (bind _returnvalue_2 (Game|SpawnActorfromClass "/Game/Enemies/BP_2DEnemy_Melee.BP_2DEnemy_Melee_C" (Math|Transform|MakeTransform _output_get "0, 0, 0" "1.000000,1.000000,1.000000") "Undefined" "MultiplyWithRoot" 0 0)))
    (:then_1
      (bind _returnvalue_3 (Game|SpawnActorfromClass "/Game/Enemies/BP_2DEnemy_Melee.BP_2DEnemy_Melee_C" (Math|Transform|MakeTransform _output_get_2 "0, 0, 0" "1.000000,1.000000,1.000000") "Undefined" "MultiplyWithRoot" 0 0))
      (Default|CallOnAttackEnd))))

(event Game|Damage|EventAnyDamage
  (params (Damage :type Float%20%28single-precision%29) (DamageType :type Damage%20Type%20Object%20Reference) (InstigatedBy :type Controller%20Object%20Reference) (DamageCauser :type Actor%20Object%20Reference))
  (bind _health (Variables|Default|GetHealth))
  (|CallParentFunction Damage 0 0 0)
  (Development|PrintString (Utilities|String|ToString(Float) _health))
  (if (<= _health 0.0)
    (Actor|DestroyActor)))

(fn ConstructionScript
  (|CallParentFunction))

(fn SetMovementSpeed
  (params (Speed :type E_MovementSpeed%20Enum :default "NewEnumerator0"))
  (bind _output_get (Variables|/Script/Engine.CharacterMovementComponent|SetMaxWalkSpeed (Variables|Character|GetCharacterMovement) (Utilities|Select :Index Speed :NewEnumerator0 0.0 :NewEnumerator1 2e+02 :NewEnumerator2 5e+02)))
  (return _output_get))

(fn GetIdealRange
  (return 4e+02 4e+02))