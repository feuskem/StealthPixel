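; NPC1 character that walks scripted paths through five WALK events, each chaining AIMoveTo calls between hard-coded world points.
; Tick maps velocity X/Y signs to a diagonal Directionality vector, while RotateCharacter derives a cardinal one in the separate Directioanlity variable.
; Helpers expose stuck detection, the patrol route and speed presets.
; ChasePlayer is empty, GetIdealRange returns zeros, and nothing here calls the walk events.
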(event Custom|WALK1
  (bind _self self)
  (AI|AIMoveTo self "-1515.230130,1433.323453,50.000000" 0 1e+02 false
    (:OnSuccess
      (AI|AIMoveTo self "-1695.230130,1653.323453,50.000000" 0 5.0 false
        (:OnSuccess
          (AI|AIMoveTo self "-1628.230130,1940.323453,50.000000" 0 1e+02 false
            (:OnSuccess
              (AI|AIMoveTo _self "-1932.230130,2238.323453,50.000000" 0 5.0 false
                (:OnSuccess
                  (AI|AIMoveTo _self "-1788.230130,2457.323453,50.000000" 0 5.0 false))))))))))

(event Custom|WALK2
  (bind _self self)
  (AI|AIMoveTo _self "-1408.230130,2759.323453,50.000000" 0 1e+02 false
    (:OnSuccess
      (AI|AIMoveTo _self "-1848.230130,3356.323453,50.000000" 0 1e+02 false
        (:OnSuccess
          (AI|AIMoveTo _self "-1960.230130,3708.323453,50.000000" 0 1e+02 false))))))

(event Custom|WALK3
  (bind _self self)
  (AI|AIMoveTo _self "-1520.230130,4018.323453,50.000000" 0 1e+02 false
    (:OnSuccess
      (AI|AIMoveTo _self "-1885.230130,4400.323453,50.000000" 0 1e+02 false
        (:OnSuccess
          (AI|AIMoveTo _self "-1476.230130,4731.323453,50.000000" 0 1e+02 false
            (:OnSuccess
              (AI|AIMoveTo _self "-886.230130,4425.323453,50.000000" 0 5.0 false
                (:OnSuccess
                  (AI|AIMoveTo _self "-499.230130,4312.323453,50.000000" 0 5.0 false))))))))))

(event Custom|WALK4
  (bind _self self)
  (AI|AIMoveTo _self "-421.230130,4683.323453,50.000000" 0 1e+02 false
    (:OnSuccess
      (AI|AIMoveTo _self "24.769870,4910.323453,50.000000" 0 1e+02 false))))

(event Custom|ChasePlayer)

(event Custom|zort)

(event Custom|WALK5
  (bind _self self)
  (AI|AIMoveTo _self "456.769870,5038.323453,50.000000" 0 1e+02 false
    (:OnSuccess
      (AI|AIMoveTo _self "1107.769870,4848.323453,50.000000" 0 1e+02 false
        (:OnSuccess
          (AI|AIMoveTo _self "1413.769870,5035.323453,50.000000" 0 1e+02 false))))))

(event EventTick
  (params (DeltaSeconds :type Float%20%28single-precision%29))
  (bind _returnvalue (Transformation|GetVelocity))
  (Utilities|FlowControl|Sequence
    (:then_0
      (Variables|Default|SetEnemyX (.x _returnvalue))
      (Variables|Default|SetEnemyY (.y _returnvalue))
      (if (and (< (Variables|Default|GetEnemyX) 0.0) (< (Variables|Default|GetEnemyY) 0.0))
        (Variables|Default|SetDirectionality (Math|Vector2D|MakeVector2D -1.0 1.0))
        (elif (and (< (Variables|Default|GetEnemyX) 0.0) (> (Variables|Default|GetEnemyY) 0.0))
          (Variables|Default|SetDirectionality (Math|Vector2D|MakeVector2D -1.0 -1.0))
          (elif (and (> (Variables|Default|GetEnemyX) 0.0) (> (Variables|Default|GetEnemyY) 0.0))
            (Variables|Default|SetDirectionality (Math|Vector2D|MakeVector2D 1.0 -1.0))
            (elif (and (> (Variables|Default|GetEnemyX) 0.0) (< (Variables|Default|GetEnemyY) 0.0))
              (Variables|Default|SetDirectionality (Math|Vector2D|MakeVector2D 1.0 1.0)))))))))

(event EventBeginPlay
  (Variables|Default|SetDirectionality (Math|Vector2D|MakeVector2D 1.0 -1.0)))

(fn ConstructionScript)

(fn IsStuck
  (return (and (Variables|Default|GetIsHoldingMove) (< (Math|Vector|VectorLength (Transformation|GetVelocity)) (Variables|Default|GetStuckTrehshlod)))))

(fn RotateCharacter
  (bind _rotationpoint (Variables|Default|GetRotationPoint))
  (bind _relativerotation (Variables|/Script/Engine.SceneComponent|GetRelativeRotation _rotationpoint))
  (if (and (< (.pitch _relativerotation) -45.0) (> (.pitch _relativerotation) -135.0))
    (Variables|Default|SetDirectioanlity "(X=0.000000,Y=-1.000000)")
    (elif (and (> (.pitch _relativerotation) 45.0) (< (.pitch _relativerotation) 135.0))
      (Variables|Default|SetDirectioanlity "(X=0.000000,Y=1.000000)")
      (elif (or (Math|Float|InRange(Float) (.roll _relativerotation) 1.6e+02 2e+02) (Math|Float|InRange(Float) (.roll _relativerotation) -2e+02 -1.6e+02))
        (Variables|Default|SetDirectioanlity "(X=-1.000000,Y=0.000000)")
        (elif (and (> (.pitch _relativerotation) -45.0) (< (.pitch _relativerotation) 45.0))
          (Variables|Default|SetDirectioanlity "(X=1.000000,Y=0.000000)"))))))

(fn GetIdealRange
  (return 0.0 0.0))

(fn GetPatrolRoute
  (return (Variables|Default|GetPatrolRoute)))

(fn SetMovementSpeed
  (params (Speed :type E_MovementSpeed%20Enum :default "NewEnumerator0"))
  (bind _output_get (Variables|/Script/Engine.CharacterMovementComponent|SetMaxWalkSpeed (Variables|Character|GetCharacterMovement) (Utilities|Select :Index Speed :NewEnumerator0 0.0 :NewEnumerator1 1e+02 :NewEnumerator2 3e+02)))
  (return _output_get))