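; Base character for 2D enemies, tracking health and a facing direction.
; Tick derives diagonal Directionality from velocity signs, while RotateCharacter sets a separate cardinal Directioanlity from RotationPoint rotation.
; Helpers provide stuck detection, patrol route, walk-speed presets and a zeroed ideal range.
; Damage lowers Health, but the zero-health branch is empty and the AIMoveTo chase and DestroyActor nodes are disconnected.
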(event Custom|ChasePlayer)

(event Custom|zort)

(event EventTick
  (params (DeltaSeconds :type Float%20%28single-precision%29))
  (bind _returnvalue (Transformation|GetVelocity))
  (Utilities|FlowControl|Sequence
    (:then_0
      (Variables|Default|SetEnemyX (.x _returnvalue))
      (Variables|Default|SetEnemyY (.y _returnvalue))
      (if (and (< (Variables|Default|GetEnemyX) 0.0) (< (Variables|Default|GetEnemyY) 0.0))
        (Variables|Default|SetDirectionality (Math|Vector2D|MakeVector2D -1.0 1.0))
        (elif (and (< (Variables|Default|GetEnemyX) 0.0) (> (Variables|Default|GetEnemyY) 0.0))
          (Variables|Default|SetDirectionality (Math|Vector2D|MakeVector2D -1.0 -1.0))
          (elif (and (> (Variables|Default|GetEnemyX) 0.0) (> (Variables|Default|GetEnemyY) 0.0))
            (Variables|Default|SetDirectionality (Math|Vector2D|MakeVector2D 1.0 -1.0))
            (elif (and (> (Variables|Default|GetEnemyX) 0.0) (< (Variables|Default|GetEnemyY) 0.0))
              (Variables|Default|SetDirectionality (Math|Vector2D|MakeVector2D 1.0 1.0)))))))
    (:then_1
      (if (<= (Variables|Default|GetHealth) 0.0)
        _))))

(event Game|Damage|EventAnyDamage
  (params (Damage :type Float%20%28single-precision%29) (DamageType :type Damage%20Type%20Object%20Reference) (InstigatedBy :type Controller%20Object%20Reference) (DamageCauser :type Actor%20Object%20Reference))
  (Variables|Default|SetHealth (- (Variables|Default|GetHealth) Damage)))

(event EventBeginPlay
  (Variables|Default|SetDirectionality (Math|Vector2D|MakeVector2D 1.0 -1.0)))

(fn ConstructionScript)

(fn IsStuck
  (return (and (Variables|Default|GetIsHoldingMove) (< (Math|Vector|VectorLength (Transformation|GetVelocity)) (Variables|Default|GetStuckTrehshlod)))))

(fn RotateCharacter
  (bind _rotationpoint (Variables|Default|GetRotationPoint))
  (bind _relativerotation (Variables|/Script/Engine.SceneComponent|GetRelativeRotation _rotationpoint))
  (if (and (< (.pitch _relativerotation) -45.0) (> (.pitch _relativerotation) -135.0))
    (Variables|Default|SetDirectioanlity "(X=0.000000,Y=-1.000000)")
    (elif (and (> (.pitch _relativerotation) 45.0) (< (.pitch _relativerotation) 135.0))
      (Variables|Default|SetDirectioanlity "(X=0.000000,Y=1.000000)")
      (elif (or (Math|Float|InRange(Float) (.roll _relativerotation) 1.6e+02 2e+02) (Math|Float|InRange(Float) (.roll _relativerotation) -2e+02 -1.6e+02))
        (Variables|Default|SetDirectioanlity "(X=-1.000000,Y=0.000000)")
        (elif (and (> (.pitch _relativerotation) -45.0) (< (.pitch _relativerotation) 45.0))
          (Variables|Default|SetDirectioanlity "(X=1.000000,Y=0.000000)"))))))

(fn GetIdealRange
  (return 0.0 0.0))

(fn GetPatrolRoute
  (return (Variables|Default|GetPatrolRoute)))

(fn SetMovementSpeed
  (params (Speed :type E_MovementSpeed%20Enum :default "NewEnumerator0"))
  (bind _output_get (Variables|/Script/Engine.CharacterMovementComponent|SetMaxWalkSpeed (Variables|Character|GetCharacterMovement) (Utilities|Select :Index Speed :NewEnumerator0 0.0 :NewEnumerator1 1e+02 :NewEnumerator2 3e+02)))
  (return _output_get))