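; Melee enemy Blueprint for a 2D character, layering damage reactions and an attack on its parent class.
; Damage triggers a hit animation and briefly sets the blackboard Hit flag; at zero health it notifies its AI controller, hides its widget, plays death and is destroyed.
; Unless the blackboard marks it disarmed, Attack applies delayed damage to TargetActor as player or decoy trap, then signals attack end.
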(event Collision|EventActorBeginOverlap
  (params (OtherActor :type Actor%20Object%20Reference)))

(event EventTick
  (params (DeltaSeconds :type Float%20%28single-precision%29))
  (|CallParentFunction DeltaSeconds))

(event EventAttack
  (bind _returnvalue (Utilities|Name|MakeLiteralName "TargetActor"))
  (bind _self self)
  (bind _returnvalue_2 (AI|GetAIController _self))
  (bind _returnvalue_3 (AI|GetBlackboard _returnvalue_2))
  (bind _returnvalue_4 (AI|Components|Blackboard|GetValueasObject _returnvalue_3 _returnvalue))
  (if (not (ScalableFloat|GetValueasBool _returnvalue_3 (Utilities|Name|MakeLiteralName "IsDisarmed")))
    (Utilities|FlowControl|Sequence
      (:then_0
        (Utilities|FlowControl|Delay 0.2)
        (bind _asbp_2dcharacter (Utilities|Casting|CastToBP_2DCharacter _returnvalue_4))
        (Game|Damage|ApplyDamage _asbp_2dcharacter 1e+01 0 0 "/Script/Engine.DamageType"))
      (:then_1
        (Utilities|FlowControl|Delay 0.2)
        (bind _asbp_decoy_trap (Utilities|Casting|CastToBp_DecoyTrap _returnvalue_4)
          (:then
            _)
          (:CastFailed
            _))
        (Game|Damage|ApplyDamage _asbp_decoy_trap 1e+01 0 0 "/Script/Engine.DamageType")))
    (Default|CallOnAttackEnd)))

(event EventBeginPlay
  (|CallParentFunction))

(event Game|Damage|EventAnyDamage
  (params (Damage :type Float%20%28single-precision%29) (DamageType :type Damage%20Type%20Object%20Reference) (InstigatedBy :type Controller%20Object%20Reference) (DamageCauser :type Actor%20Object%20Reference))
  (bind _self self)
  (bind _returnvalue (AI|GetAIController _self))
  (bind _returnvalue_2 (AI|GetBlackboard _returnvalue))
  (|CallParentFunction Damage 0 0 0)
  (if (<= (Variables|Default|GetHealth) 0.0)
    (bind _asaic_enemy_base (Utilities|Casting|CastToAIC_Enemy_Base (Pawn|GetController)))
    (Default|Killed _asaic_enemy_base)
    (Development|SetHiddeninGame (Variables|Default|GetWidget) true false)
    (Class|PaperZDAnimInstance|JumptoNode (Variables|/Script/PaperZD.PaperZDAnimationComponent|GetAnimInstance (Variables|Default|GetAnimationComponent)) "DeathJ" "None")
    (Utilities|FlowControl|Delay 2.0)
    (Actor|DestroyActor)
    (else
      (Class|PaperZDAnimInstance|JumptoNode (Variables|/Script/PaperZD.PaperZDAnimationComponent|GetAnimInstance (Variables|Default|GetAnimationComponent)) "HitR" "None")
      (AI|Components|Blackboard|SetValueasBool _returnvalue_2 (Utilities|Name|MakeLiteralName "Hit") true)
      (Utilities|FlowControl|Delay 0.5)
      (AI|Components|Blackboard|SetValueasBool _returnvalue_2 (Utilities|Name|MakeLiteralName "Hit") false))))

(fn ConstructionScript
  (|CallParentFunction))