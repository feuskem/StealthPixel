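; Ranged enemy Blueprint for a 2D enemy that attacks with fireballs and destroys itself when its health runs out.
; Attack waits briefly, checks that the AI controller has a valid target, then spawns a fireball aimed at the player pawn rather than that target, and signals attack end.
; It also maps movement speed states to walk speed and reports ideal attack and defend ranges.
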(event EventBeginPlay
  (|CallParentFunction) ; This node is disabled and will not be called.\nDrag off pins to build functionality.
)

(event Collision|EventActorBeginOverlap
  (params (OtherActor :type Actor%20Object%20Reference)))

(event EventTick
  (params (DeltaSeconds :type Float%20%28single-precision%29)))

(event EventAttack
  (bind _returnvalue (Transformation|GetActorLocation))
  (Utilities|FlowControl|Delay 0.2)
  (bind _asaic_enemy_base (Utilities|Casting|CastToAIC_Enemy_Base (AI|GetAIController self)))
  (bind _attack_target (Variables|/Game/Enemies/AI/AIC_Enemy_Base.AIC_Enemy_Base_C|GetAttack%20Target _asaic_enemy_base)
    (:then
      (Game|SpawnActorfromClass "/Game/Enemies/Fireball.Fireball_C" (Math|Transform|MakeTransform _returnvalue (Math|Rotator|FindLookatRotation _returnvalue (Transformation|GetActorLocation (Game|Player|GetPlayerPawn 0))) "1.000000,1.000000,1.000000") "Undefined" "MultiplyWithRoot" self 0)
      (Default|CallOnAttackEnd))
    (:else
      (Development|PrintString "GÜM"))))

(event Game|Damage|EventAnyDamage
  (params (Damage :type Float%20%28single-precision%29) (DamageType :type Damage%20Type%20Object%20Reference) (InstigatedBy :type Controller%20Object%20Reference) (DamageCauser :type Actor%20Object%20Reference))
  (|CallParentFunction Damage 0 0 0)
  (if (<= (Variables|Default|GetHealth) 0.0)
    (Actor|DestroyActor)))

(fn ConstructionScript
  (|CallParentFunction))

(fn SetMovementSpeed
  (params (Speed :type E_MovementSpeed%20Enum :default "NewEnumerator0"))
  (bind _output_get (Variables|/Script/Engine.CharacterMovementComponent|SetMaxWalkSpeed (Variables|Character|GetCharacterMovement) (Utilities|Select :Index Speed :NewEnumerator0 0.0 :NewEnumerator1 2e+02 :NewEnumerator2 5e+02)))
  (return _output_get))

(fn GetIdealRange
  (return 4e+02 4e+02))