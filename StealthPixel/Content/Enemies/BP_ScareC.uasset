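; BP_ScareC is an enemy Blueprint that serves as a tutorial target, advancing the player's combat tutorial when killed.
; Each Tick it checks whether Health is zero or below, then casts the player pawn to BP_2DCharacter.
; It sets the first incomplete flag in melee, ranged, stealth order, regardless of how it died, then destroys itself.
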(event EventBeginPlay
  (|CallParentFunction) ; This node is disabled and will not be called.\nDrag off pins to build functionality.
)

(event Collision|EventActorBeginOverlap
  (params (OtherActor :type Actor%20Object%20Reference)))

(event EventTick
  (params (DeltaSeconds :type Float%20%28single-precision%29))
  (|CallParentFunction DeltaSeconds)
  (if (<= (Variables|Default|GetHealth) 0.0)
    (bind _asbp_2dcharacter (Utilities|Casting|CastToBP_2DCharacter (Game|Player|GetPlayerPawn 0)))
    (if (Variables|/Game/Character/BP_2DCharacter.BP_2DCharacter_C|GetHasCompletedMeeleTut _asbp_2dcharacter)
      (if (Variables|/Game/Character/BP_2DCharacter.BP_2DCharacter_C|GetHasCompletedRangedTut _asbp_2dcharacter)
        (Variables|/Game/Character/BP_2DCharacter.BP_2DCharacter_C|SetHasCompletedStealthTut _asbp_2dcharacter true)
        (Actor|DestroyActor)
        (else
          (Variables|/Game/Character/BP_2DCharacter.BP_2DCharacter_C|SetHasCompletedRangedTut _asbp_2dcharacter true)
          (Actor|DestroyActor)))
      (else
        (Variables|/Game/Character/BP_2DCharacter.BP_2DCharacter_C|SetHasCompletedMeeleTut _asbp_2dcharacter true)
        (Actor|DestroyActor)))))

(fn ConstructionScript
  (|CallParentFunction))