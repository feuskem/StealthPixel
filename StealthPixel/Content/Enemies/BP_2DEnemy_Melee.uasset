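; Melee enemy for a 2D game that damages the player character and dies when its health runs out.
; AnyDamage lowers Health, while Tick prints it for debugging and destroys the actor at zero or below.
; Attack waits briefly, casts the AI blackboard's TargetActor to BP_2DCharacter, applies damage and calls OnAttackEnd.
; A failed cast only prints a debug message, so OnAttackEnd is not called.
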(event EventBeginPlay
  (|CallParentFunction) ; This node is disabled and will not be called.\nDrag off pins to build functionality.
)

(event Collision|EventActorBeginOverlap
  (params (OtherActor :type Actor%20Object%20Reference)))

(event EventTick
  (params (DeltaSeconds :type Float%20%28single-precision%29))
  (bind _health (Variables|Default|GetHealth))
  (Development|PrintString (Utilities|String|ToString(Float) _health))
  (if (<= _health 0.0)
    (Actor|DestroyActor)))

(event EventAttack
  (Development|PrintString "SD")
  (Utilities|FlowControl|Delay 0.2)
  (bind _asbp_2dcharacter (Utilities|Casting|CastToBP_2DCharacter (AI|Components|Blackboard|GetValueasObject (AI|GetBlackboard (AI|GetAIController self)) (Utilities|Name|MakeLiteralName "TargetActor")))
    (:then
      (Game|Damage|ApplyDamage _asbp_2dcharacter 1e+01 0 0 "/Script/Engine.DamageType")
      (Default|CallOnAttackEnd))
    (:CastFailed
      (Development|PrintString "Vuramadım abi"))))

(event Game|Damage|EventAnyDamage
  (params (Damage :type Float%20%28single-precision%29) (DamageType :type Damage%20Type%20Object%20Reference) (InstigatedBy :type Controller%20Object%20Reference) (DamageCauser :type Actor%20Object%20Reference))
  (Variables|Default|SetHealth (- (Variables|Default|GetHealth) Damage)))

(fn ConstructionScript
  (|CallParentFunction))