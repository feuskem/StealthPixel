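; BP_CommonArrow is a 2D arrow projectile that damages BP_2DEnemyBase actors through its Sphere overlap, then destroys itself.
; Its flipbook is unhidden shortly after spawn, and the arrow expires a few seconds later.
; Three hit colliders each roll independently for a one-in-three chance to stop it, while a fourth always stops it; stopped arrows are destroyed after a brief delay.
; Gravity logic is unwired.
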(event OnComponentBeginOverlap(Hİt)
  (params (OverlappedComponent :type Primitive%20Component%20Object%20Reference) (OtherActor :type Actor%20Object%20Reference) (OtherComp :type Primitive%20Component%20Object%20Reference) (OtherBodyIndex :type Integer) (bFromSweep :type Boolean) (SweepResult :type Hit%20Result%20Structure%20%28by%20ref%29))
  (switch int (Math|Conversions|ToInteger(Byte) (Class|KismetMathLibrary|RandomInteger64inRange 0 2))
    (:0
      (Game|Components|ProjectileMovement|SetVelocityinLocalSpace (Variables|Default|GetProjectileMovement) "0, 0, 0")
      (Utilities|FlowControl|Delay 0.5)
      (Actor|DestroyActor))))

(event OnComponentBeginOverlap(Hİt1)
  (params (OverlappedComponent :type Primitive%20Component%20Object%20Reference) (OtherActor :type Actor%20Object%20Reference) (OtherComp :type Primitive%20Component%20Object%20Reference) (OtherBodyIndex :type Integer) (bFromSweep :type Boolean) (SweepResult :type Hit%20Result%20Structure%20%28by%20ref%29))
  (switch int (Math|Conversions|ToInteger(Byte) (Class|KismetMathLibrary|RandomInteger64inRange 0 2))
    (:1
      (Game|Components|ProjectileMovement|SetVelocityinLocalSpace (Variables|Default|GetProjectileMovement) "0, 0, 0")
      (Utilities|FlowControl|Delay 0.5)
      (Actor|DestroyActor))))

(event OnComponentBeginOverlap(Hİt2)
  (params (OverlappedComponent :type Primitive%20Component%20Object%20Reference) (OtherActor :type Actor%20Object%20Reference) (OtherComp :type Primitive%20Component%20Object%20Reference) (OtherBodyIndex :type Integer) (bFromSweep :type Boolean) (SweepResult :type Hit%20Result%20Structure%20%28by%20ref%29))
  (switch int (Math|Conversions|ToInteger(Byte) (Class|KismetMathLibrary|RandomInteger64inRange 0 2))
    (:2
      (Game|Components|ProjectileMovement|SetVelocityinLocalSpace (Variables|Default|GetProjectileMovement) "0, 0, 0")
      (Utilities|FlowControl|Delay 0.5)
      (Actor|DestroyActor))))

(event OnComponentBeginOverlap(Sphere)
  (params (OverlappedComponent :type Primitive%20Component%20Object%20Reference) (OtherActor :type Actor%20Object%20Reference) (OtherComp :type Primitive%20Component%20Object%20Reference) (OtherBodyIndex :type Integer) (bFromSweep :type Boolean) (SweepResult :type Hit%20Result%20Structure%20%28by%20ref%29))
  (bind _asbp_2denemy_base (Utilities|Casting|CastToBP_2DEnemyBase OtherActor)
    (:then
      (Game|Damage|ApplyDamage _asbp_2denemy_base 5e+01 0 0 "/Script/Engine.DamageType")
      (Actor|DestroyActor))
    (:CastFailed
      (Development|PrintString "Neden acaba"))))

(event OnComponentBeginOverlap(Hİt3)
  (params (OverlappedComponent :type Primitive%20Component%20Object%20Reference) (OtherActor :type Actor%20Object%20Reference) (OtherComp :type Primitive%20Component%20Object%20Reference) (OtherBodyIndex :type Integer) (bFromSweep :type Boolean) (SweepResult :type Hit%20Result%20Structure%20%28by%20ref%29))
  (Game|Components|ProjectileMovement|SetVelocityinLocalSpace (Variables|Default|GetProjectileMovement) "0, 0, 0")
  (Utilities|FlowControl|Delay 0.5)
  (Actor|DestroyActor))

(event Custom|gravity)

(event EventBeginPlay
  (Utilities|FlowControl|Delay 0.2)
  (Development|SetHiddeninGame (Variables|Default|GetPaperFlipbook) false false)
  (Utilities|FlowControl|Delay 4.0)
  (Actor|DestroyActor))

(event Collision|EventActorBeginOverlap
  (params (OtherActor :type Actor%20Object%20Reference)))

(event EventTick
  (params (DeltaSeconds :type Float%20%28single-precision%29)))

(fn ConstructionScript)