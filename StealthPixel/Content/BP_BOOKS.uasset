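; BP_BOOKS is a trigger actor that ends the level by loading the Menu once the player has both books.
; Its two flipbooks start stopped and hidden.
; When a BP_2DCharacter with both BOOK1 and BOOK2 set overlaps the Box, both flipbooks appear and play briefly.
; Timed delays stop the animation, then open the Menu level.
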(event OnComponentBeginOverlap(Box)
  (params (OverlappedComponent :type Primitive%20Component%20Object%20Reference) (OtherActor :type Actor%20Object%20Reference) (OtherComp :type Primitive%20Component%20Object%20Reference) (OtherBodyIndex :type Integer) (bFromSweep :type Boolean) (SweepResult :type Hit%20Result%20Structure%20%28by%20ref%29))
  (bind _asbp_2dcharacter (Utilities|Casting|CastToBP_2DCharacter OtherActor))
  (if (and (Variables|/Game/Character/BP_2DCharacter.BP_2DCharacter_C|GetBOOK1 _asbp_2dcharacter) (Variables|/Game/Character/BP_2DCharacter.BP_2DCharacter_C|GetBOOK2 _asbp_2dcharacter))
    (Rendering|SetVisibility (Variables|Default|GetPaperFlipbook1) true false)
    (Audio|Components|Audio|Play (Variables|Default|GetPaperFlipbook1))
    (Utilities|FlowControl|Delay 0.6)
    (Audio|Components|Audio|Stop (Variables|Default|GetPaperFlipbook1))
    (Utilities|FlowControl|Delay 0.3)
    (Game|OpenLevel(byName) "Menu")))

(event EventBeginPlay
  (Audio|Components|Audio|Stop (Variables|Default|GetPaperFlipbook))
  (Rendering|SetVisibility (Variables|Default|GetPaperFlipbook) false false))

(event Collision|EventActorBeginOverlap
  (params (OtherActor :type Actor%20Object%20Reference)))

(event EventTick
  (params (DeltaSeconds :type Float%20%28single-precision%29)))

(fn ConstructionScript)